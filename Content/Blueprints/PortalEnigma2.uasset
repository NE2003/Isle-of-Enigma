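; PortalEnigma2 is a portal puzzle actor that loads the Cave level once the player has taken the pillar key.
; The Box1 trigger enables input and shows the PickUp prompt; pressing E there hides the key and prompt via transparent materials, plays a switch sound and sets Finished.
; The Box trigger opens the level when finished, otherwise shows MissingKey, which hides ten seconds after the player leaves.
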(event `self.Box1.OnComponentBeginOverlap`
  (params (OverlappedComponent :type "PrimitiveComponent Object Reference") (OtherActor :type "Actor Object Reference") (OtherComp :type "PrimitiveComponent Object Reference") (OtherBodyIndex :type Integer) (bFromSweep :type Boolean) (SweepResult :type "HitResult Structure (by ref)"))
  (set `self.BoxNumber` 1)
  (cast `/Game/Player/BP_PlayerCharacter` OtherActor)
  (`self.EnableInput` (`GameplayStatics.GetPlayerController` 0))
  (`SceneComponent.SetVisibility` (`self.Pick up`) true false))

(event `self.Box.OnComponentBeginOverlap`
  (params (OverlappedComponent :type "PrimitiveComponent Object Reference") (OtherActor :type "Actor Object Reference") (OtherComp :type "PrimitiveComponent Object Reference") (OtherBodyIndex :type Integer) (bFromSweep :type Boolean) (SweepResult :type "HitResult Structure (by ref)"))
  (if (`KismetMathLibrary.Conv_IntToBool` (`self.Finished!`))
    (cast `PlayerCharacter` OtherActor)
    (`GameplayStatics.OpenLevel` "Cave")
    (else
      (`SceneComponent.SetVisibility` (`self.Missing Key`) true false))))

(event `self.Box1.OnComponentEndOverlap`
  (params (OverlappedComponent :type "PrimitiveComponent Object Reference") (OtherActor :type "Actor Object Reference") (OtherComp :type "PrimitiveComponent Object Reference") (OtherBodyIndex :type Integer))
  (cast `/Game/Player/BP_PlayerCharacter` OtherActor)
  (`self.DisableInput` (`GameplayStatics.GetPlayerController` 0) null)
  (`SceneComponent.SetVisibility` (`self.Pick up`) false false))

(event `self.Box.OnComponentEndOverlap`
  (params (OverlappedComponent :type "PrimitiveComponent Object Reference") (OtherActor :type "Actor Object Reference") (OtherComp :type "PrimitiveComponent Object Reference") (OtherBodyIndex :type Integer))
  (cast `PlayerCharacter` OtherActor)
  (`KismetSystemLibrary.Delay` 10.0)
  (`SceneComponent.SetVisibility` (`self.Missing Key`) false false))

(event `Key|E`
  (params (Key :type "Key Structure"))
  (:`Pressed`
    (if (`KismetStringLibrary.EqualEqual_StrStr` (`KismetStringLibrary.Conv_IntToString` (`self.BoxNumber`)) (`KismetStringLibrary.Conv_IntToString` 1))
      (`PrimitiveComponent.SetMaterial` (`self.PillarKey`) 0 "/Game/Materials/TransparentMaterial.TransparentMaterial")
      (`GameplayStatics.PlaySoundAtLocation` "/Game/Sound/runestone/Bluezone_BC0302_industrial_lever_switch_small_003.Bluezone_BC0302_industrial_lever_switch_small_003" (`SceneComponent.K2_GetComponentLocation` (`self.PillarKey`)) (struct) 1.0 1.0 0.0 null null null null)
      (`PrimitiveComponent.SetCollisionEnabled` (`self.PillarKey`) "NoCollision")
      (`PrimitiveComponent.SetMaterial` (`self.Pick up`) 0 "/Game/Materials/TransparentMaterial.TransparentMaterial")
      (set `self.Finished!` 1))))

(fn `UserConstructionScript`)