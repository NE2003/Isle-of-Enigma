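; Blueprint function library that feeds a spotlight's cone shape into MPC_SpotlightReveal, presumably for materials that reveal surfaces under the light.
; It writes the light's location as StartSpot and its attenuation radius, then line-traces forward for EndSpot, falling back to full range on a miss.
; Radius at EndSpot comes from distance times the tangent of the outer cone angle; a hidden light collapses the cone to zero.
; One collection serves only one spotlight.
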(fn `SpotlightReveal`
  (params (Spotlight :type "SpotLightComponent Object Reference"))
  (bind _returnvalue (`SceneComponent.K2_GetComponentLocation` Spotlight))
  (bind _attenuationradius (`LocalLightComponent.AttenuationRadius` Spotlight))
  (bind _returnvalue_2 (`KismetMathLibrary.DegTan` (`SpotLightComponent.OuterConeAngle` Spotlight)))
  (bind _returnvalue_3 (+ _returnvalue (* (`SceneComponent.GetForwardVector` Spotlight) (`LocalLightComponent.AttenuationRadius` Spotlight))))
  ;[1 1 1] It's important to pass the correct values to the correct Material Parameter Collection for each Spotlight. One MPC works only for one specific Spotlight.
  (`KismetMaterialLibrary.SetScalarParameterValue` null "/Game/SpotlightReveal/Materials/MPC_SpotlightReveal.MPC_SpotlightReveal" "Attenuation" (`LocalLightComponent.AttenuationRadius` Spotlight))
  (`KismetMaterialLibrary.SetVectorParameterValue` null "/Game/SpotlightReveal/Materials/MPC_SpotlightReveal.MPC_SpotlightReveal" "StartSpot" (`KismetMathLibrary.Conv_VectorToLinearColor` _returnvalue))
  ;[1 1 1] If the Spotlight is not visible, it's off and different values should be passed to EndSpot and Radius.
  (if (`SceneComponent.IsVisible` Spotlight)
    ;[1 1 1] A line trace is used to determine the point where the spotlight hits.
    (bind (_outhit _returnvalue_4) (`KismetSystemLibrary.LineTraceSingle` null (`SceneComponent.K2_GetComponentLocation` Spotlight) _returnvalue_3 "TraceTypeQuery1"))
    (if _returnvalue_4
      (bind (_bblockinghit _binitialoverlap _time _distance _location _impactpoint) (`GameplayStatics.BreakHitResult` _outhit))
      ;[1 1 1] The EndSpot value is the impact point where the Spotlight hits. If the Spotlight is not visible, the EndSpot is the same as the StartSpot.
      (`KismetMaterialLibrary.SetVectorParameterValue` null "/Game/SpotlightReveal/Materials/MPC_SpotlightReveal.MPC_SpotlightReveal" "EndSpot" (`KismetMathLibrary.Conv_VectorToLinearColor` _impactpoint))
      ;[1 1 1] Since the Spotlight has the shape of a cone, the Radius at the impact point is determined by the formula:
      ; radius = height * tan(angle)
      ; The height of the Spotlight's cone is the same as its Attenuation Radius, and the angle is the same as the Outer Cone's angle.  If the Spotlight is not visible, the Radius is 0.
      (`KismetMaterialLibrary.SetScalarParameterValue` null "/Game/SpotlightReveal/Materials/MPC_SpotlightReveal.MPC_SpotlightReveal" "Radius" (* (`KismetMathLibrary.FClamp` (`KismetMathLibrary.VSize` (- _impactpoint (`SceneComponent.K2_GetComponentLocation` Spotlight))) 0.0 _attenuationradius) _returnvalue_2))
      (else
        (`KismetMaterialLibrary.SetVectorParameterValue` null "/Game/SpotlightReveal/Materials/MPC_SpotlightReveal.MPC_SpotlightReveal" "EndSpot" (`KismetMathLibrary.Conv_VectorToLinearColor` _returnvalue_3))
        (`KismetMaterialLibrary.SetScalarParameterValue` null "/Game/SpotlightReveal/Materials/MPC_SpotlightReveal.MPC_SpotlightReveal" "Radius" (* _attenuationradius _returnvalue_2))))
    (else
      (`KismetMaterialLibrary.SetVectorParameterValue` null "/Game/SpotlightReveal/Materials/MPC_SpotlightReveal.MPC_SpotlightReveal" "EndSpot" (`KismetMathLibrary.Conv_VectorToLinearColor` (`SceneComponent.K2_GetComponentLocation` Spotlight)))
      (`KismetMaterialLibrary.SetScalarParameterValue` null "/Game/SpotlightReveal/Materials/MPC_SpotlightReveal.MPC_SpotlightReveal" "Radius"))))